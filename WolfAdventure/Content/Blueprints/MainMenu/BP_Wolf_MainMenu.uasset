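; BP_Wolf_MainMenu is the animated main menu display with a staff, fireball and magic circle decal.
; On BeginPlay it starts the menu music, shows WBP_MainMenu with UI-only input and mouse cursor, and caches the prop locations.
; Each Tick it spins the staff and decal, and bobs staff and fireball vertically around those cached locations using a shared sine timer that resets after 2π.
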(event EventBeginPlay
  (bind _returnvalue (Game|GetPlayerController 0))
  (Variables|Default|SetFireballInitialLocation (Transformation|GetWorldLocation (Variables|Default|GetFireball)))
  (Variables|Default|SetStaffInitialLocation (Transformation|GetWorldLocation (Variables|Default|GetStaff)))
  (bind _returnvalue_2 (Audio|SpawnSound2D "/Game/Assets/Sounds/Music/Music_MainMenu.Music_MainMenu" 1.0 1.0 0.0 0))
  (Variables|Default|SetMainMenuMusic _returnvalue_2)
  (bind _returnvalue_3 (UserInterface|CreateWidget "/Game/Blueprints/UI/MainMenu/WBP_MainMenu.WBP_MainMenu_C"))
  (UserInterface|Viewport|AddtoViewport _returnvalue_3 0)
  (Input|SetInputModeUIOnly _returnvalue _returnvalue_3 "DoNotLock" false)
  (Variables|/Script/Engine.PlayerController|SetbShowMouseCursor _returnvalue true))

(event Collision|EventActorBeginOverlap
  (params (OtherActor :type Actor%20Object%20Reference)))

(event EventTick
  (params (DeltaSeconds :type Float%20%28single-precision%29))
  (Transformation|AddLocalRotation (Variables|Default|GetStaff) (Math|Rotator|MakeRotator 0.0 0.0 (* DeltaSeconds 12.0)) false false)
  (CallFunction|UpdateTime DeltaSeconds)
  (Transformation|SetWorldLocation (Variables|Default|GetFireball) (+ (Variables|Default|GetFireballInitialLocation) (Math|Vector|MakeVector 0.0 0.0 (CallFunction|SinTime))) false false)
  (Transformation|SetWorldLocation (Variables|Default|GetStaff) (+ (Variables|Default|GetStaffInitialLocation) (Math|Vector|MakeVector 0.0 0.0 (CallFunction|SinTime))) false false)
  (Transformation|AddLocalRotation (Variables|Default|GetMagicCircleDecal) (Math|Rotator|MakeRotator (* (Utilities|Time|GetWorldDeltaSeconds) (Variables|Default|GetMagicCircleRotationRate)) 0.0 0.0) false false))

(fn ConstructionScript)

(fn UpdateTime
  (params (Delta%20Seconds :type Float%20%28double-precision%29))
  (bind _output_get (Variables|Default|SetTime (+ Delta%20Seconds (Variables|Default|GetTime))))
  (if (> _output_get 6.28318)
    (Variables|Default|SetTime 0.0)))

(fn SinTime
  (return (* (Math|Trig|Sin(Radians) (Variables|Default|GetTime)) (Variables|Default|GetAmplitude))))