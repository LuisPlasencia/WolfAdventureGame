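; GA_FireBolt is the Wolf's Fire Bolt gameplay ability, which casts a projectile at the location under the mouse.
; On valid cursor target data it faces the avatar to the target through CombatInterface and plays the cast montage.
; A montage gameplay event triggers SpawnProjectile from the weapon socket, so the shot syncs with the animation.
; It also draws a debug sphere at the target, then ends the ability after a short delay.
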(event Ability|EventActivateAbility
  (bind _datahandle (|TargetDataUnderMouse)
    (:ValidData
      (Variables|Default|SetProjectileTargetLocation (.Location (Collision|BreakHitResult (Ability|TargetData|GetHitResultfromTargetData _datahandle))))
      (bind _ascombat_interface (Utilities|Casting|CastToCombatInterface (Ability|GetAvatarActorfromActorInfo)))
      (Class|CombatInterface|UpdateFacingTarget _ascombat_interface (Variables|Default|GetProjectileTargetLocation))
      (|PlayMontageandWaitProxy "None" "/Game/Blueprints/Characters/Animations/AM_Wolf_CastFireBolt.AM_Wolf_CastFireBolt" 1.0 "None" true 1.0 0.0 false
        (:then
          (Ability|Tasks|WaitGameplayEvent "(TagName=\"Event.Montage.FireBolt\")" 0
            (:EventReceived
              (Class|BaseProjectileSpell|SpawnProjectile (Variables|Default|GetProjectileTargetLocation) (GameplayTags|MakeLiteralGameplayTag "(TagName=\"CombatSocket.Weapon\")"))
              (Rendering|Debug|DrawDebugSphere (Variables|Default|GetProjectileTargetLocation) 1e+02 12 "(R=1.000000,G=1.000000,B=1.000000,A=1.000000)" 2e+01)
              (Utilities|FlowControl|Delay 0.5)
              (Ability|EndAbility))))))))

(event Ability|EventOnEndAbility
  (params (bWasCancelled :type Boolean)))